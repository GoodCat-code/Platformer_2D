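; BP_CarDraft is an actor, apparently a draft car, that travels along the spline of a referenced Path actor.
; On BeginPlay it calls StartMoving, which plays a timeline whose Alpha is lerped to a distance between zero and the spline's length.
; Each update sets the actor's location and rotation from the world-space spline transform at that distance.
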(event Custom|StartMoving
  (bind _alpha (Timeline|Timeline Play)
    (:Update
      (Transformation|SetActorLocationAndRotation (.location (Spline|GetTransformatDistanceAlongSpline (Variables|/Game/Bartender/Blueprints/BP_Path_for_moving_objects.BP_Path_for_moving_objects_C|GetSpline (Variables|Default|GetPath)) (Math|Float|Lerp 0.0 (Spline|GetSplineLength (Variables|/Game/Bartender/Blueprints/BP_Path_for_moving_objects.BP_Path_for_moving_objects_C|GetSpline (Variables|Default|GetPath))) _alpha) "World" false)) (.rotation (Spline|GetTransformatDistanceAlongSpline (Variables|/Game/Bartender/Blueprints/BP_Path_for_moving_objects.BP_Path_for_moving_objects_C|GetSpline (Variables|Default|GetPath)) (Math|Float|Lerp 0.0 (Spline|GetSplineLength (Variables|/Game/Bartender/Blueprints/BP_Path_for_moving_objects.BP_Path_for_moving_objects_C|GetSpline (Variables|Default|GetPath))) _alpha) "World" false))))))

(event EventBeginPlay
  (Variables|Default|SetPath (Variables|Default|GetPath))
  (CallFunction|StartMoving))

(event Collision|EventActorBeginOverlap
  (params (OtherActor :type Actor%20Object%20Reference)))

(event EventTick
  (params (DeltaSeconds :type Float%20%28single-precision%29)))

(fn ConstructionScript)
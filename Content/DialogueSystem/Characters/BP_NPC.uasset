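; Example NPC that drives story dialogue through its BPacDialogue component and exposes an interact type.
; StartDialogue shows the DataTable row for SaveScene, with cinematic mode also locking look input and playing an async-loaded Level Sequence keyed by SaveCinematic.
; Finishing increments the row name's numeric suffix while rows exist, otherwise using hard-coded transitions, as do option selection and skipping.
; Progress starts from hard-coded placeholders for save data.
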(event EventBeginPlay
  ;[1 1 1] Prepare loading save file data
  (Variables|Default|SetSaveScene "Scene1.0") ; (example) Save File: user progression of story dialogue.
  (Variables|Default|SetSaveCinematic "Cine1.0") ; (example) Save File: user progression of story dialogue for sequencer.
  (Variables|/Game/DialogueSystem/ActorComponent_Dialogue/BPac_Dialogue.BPac_Dialogue_C|SetNPC_Mesh (Variables|Default|GetBPac_Dialogue) (Variables|Default|GetSkeletalMesh)) ; Assign mesh for playing Animation
)

(event EventStartDialogue
  ;[1 1 1] Example of a scene dialogue flow
  (switch name (Variables|Default|GetTypeScene) ; To switch between Sequencer(Cinematic) or not
    (:AnimVoice
      (bind _returnvalue (Utilities|GetDataTableRow "/Game/DialogueSystem/Characters/DataTable/A1D1/DT_Mq_A1D1.DT_Mq_A1D1" (Variables|Default|GetSaveScene))
        (:then
          (Default|DisplayText (Variables|/Game/DialogueSystem/ActorComponent_Dialogue/BPac_Dialogue.BPac_Dialogue_C|GetDialogueUI (Variables|Default|GetBPac_Dialogue)) _returnvalue))))
    (:Cinematic
      (Input|SetIgnoreLookInput (Game|GetPlayerController 0) true)
      (if (not (Variables|Default|GetbSequencerLoading)) ; still loading
        (bind _returnvalue_2 (Utilities|GetDataTableRow "/Game/DialogueSystem/Sequencer/DT_Sequencer_D1.DT_Sequencer_D1" (Variables|Default|GetSaveCinematic)) ; Sequencer for cinematic
          (:then
            (Utilities|IsValid (Utilities|ResolveSoftReference (.levelsequence _returnvalue_2)) ; is already loaded
              (:Is%20Valid
                (Variables|Default|SetbSequencerLoading false :!label _label)
                (Default|PlaySequencer (Variables|Default|GetBPac_Dialogue) (Utilities|ResolveSoftReference (.levelsequence _returnvalue_2)))
                (bind _returnvalue_3 (Utilities|GetDataTableRow "/Game/DialogueSystem/Characters/DataTable/A1D1/DT_Mq_A1D1.DT_Mq_A1D1" (Variables|Default|GetSaveScene))
                  (:then
                    (Default|DisplayText (Variables|/Game/DialogueSystem/ActorComponent_Dialogue/BPac_Dialogue.BPac_Dialogue_C|GetDialogueUI (Variables|Default|GetBPac_Dialogue)) _returnvalue_3))))
              (:Is%20Not%20Valid
                (Utilities|AsyncLoadAsset (.levelsequence _returnvalue_2)
                  (:then
                    (Variables|Default|SetbSequencerLoading true))
                  (:Completed
                    (goto _label)))))))))))

(event EventSelectedOption
  (params (OptionText :type Text))
  ;[1 1 1] Example of a finish dialogue and option
  (switch name (Variables|Default|GetSaveScene)
    (:Scene1.1
      (switch string (Utilities|String|ToString(Text) OptionText)
        (:Yes
          (Variables|Default|SetSaveScene "Scene1.3")
          (Variables|Default|SetSaveCinematic "Cine1.1")
          (Class|BPIInteractTalkInterface|StartTalk(Message) (Variables|Default|GetBPac_Dialogue)))))))

(event EventFinishedDialogue
  ;[1 1 1] Example of a finish dialogue and option
  (bind _returnvalue (Class|DataTableFunctionLibrary|DoesDataTableRowExist "/Game/DialogueSystem/Characters/DataTable/A1D1/DT_Mq_A1D1.DT_Mq_A1D1" (Utilities|String|StringToName (Utilities|String|BuildString(Integer) (.LeftS (Utilities|String|Split (Utilities|String|ToString(Name) (Variables|Default|GetSaveScene)) "." "IgnoreCase" "FromEnd")) "." (+ (Math|Conversions|ToInteger(Byte) (.RightS (Utilities|String|Split (Utilities|String|ToString(Name) (Variables|Default|GetSaveScene)) "." "IgnoreCase" "FromEnd"))) 1)))))
  (if _returnvalue
    (Variables|Default|SetSaveScene (Utilities|String|StringToName (Utilities|String|BuildString(Integer) (.LeftS (Utilities|String|Split (Utilities|String|ToString(Name) (Variables|Default|GetSaveScene)) "." "IgnoreCase" "FromEnd")) "." (+ (Math|Conversions|ToInteger(Byte) (.RightS (Utilities|String|Split (Utilities|String|ToString(Name) (Variables|Default|GetSaveScene)) "." "IgnoreCase" "FromEnd"))) 1))))
    (Class|BPIInteractTalkInterface|StartTalk(Message) (Variables|Default|GetBPac_Dialogue)) ; resume dialogue
    (else
      (switch name (Variables|Default|GetSaveScene)
        (:Scene1.0
          (Variables|Default|SetSaveScene "Scene1.1"))
        (:Scene1.2
          (Variables|Default|SetSaveScene "Scene1.3"))
        (:Scene1.4
          (Variables|Default|SetSaveScene "Scene1.5"))))))

(event EventSkipDialogue
  ;[1 1 1] Example of a finish dialogue and option
  (switch name (Utilities|String|StringToName (.LeftS (Utilities|String|Split (Utilities|String|ToString(Name) (Variables|Default|GetSaveScene)) "." "IgnoreCase" "FromEnd"))) ; example: get main chapter number
    (:Scene1
      (Variables|Default|SetSaveScene "Scene1.1")
      (Class|BPIInteractTalkInterface|StartTalk(Message) (Variables|Default|GetBPac_Dialogue)))))

(fn ConstructionScript)

(fn GetInteractType
  (return (Variables|Default|GetInteract%20Type)))
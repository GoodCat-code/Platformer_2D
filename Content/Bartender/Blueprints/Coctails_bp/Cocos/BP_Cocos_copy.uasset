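; Coconut cocktail actor thrown by the side-scroller character that it can mount and ride.
; An invisible-style Cube follows the top of the physics ball each tick; overlapping it snaps the character on, pins their location, zeroes velocity and swaps input to the Cocos mapping context.
; When enchanted it launches sideways with an outside force.
; A retriggerable delay, refreshed while ridden, destroys it after its lifetime.
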(event OnComponentBeginOverlap(Cube)
  (params (OverlappedComponent :type Primitive%20Component%20Object%20Reference) (OtherActor :type Actor%20Object%20Reference) (OtherComp :type Primitive%20Component%20Object%20Reference) (OtherBodyIndex :type Integer) (bFromSweep :type Boolean) (SweepResult :type Hit%20Result%20Structure%20%28by%20ref%29))
  (bind _returnvalue (Game|GetPlayerController 0))
  (bind _throw_params (Variables|Default|GetThrow_Params))
  (bind _throw_params_2 (Variables|Default|GetThrow_Params))
  (bind _asbp_side_scroller_character (Utilities|Casting|CastToBP_SideScrollerCharacter (.main_character _throw_params)))
  (bind _asbp_side_scroller_character_2 (Utilities|Casting|CastToBP_SideScrollerCharacter (.main_character _throw_params_2)))
  (bind _returnvalue_2 (PlayerController|LocalPlayerSubsystems|GetEnhancedInputLocalPlayerSubsystem _returnvalue))
  (if (== OtherActor _asbp_side_scroller_character_2)
    ;[1 1 1] For correct functionality of coconut
    (Collision|SetCollisionEnabled (Variables|/Script/Engine.Character|GetCapsuleComponent _asbp_side_scroller_character_2) "NoCollision")
    (Collision|SetCollisionEnabled (Variables|/Script/Engine.Character|GetMesh _asbp_side_scroller_character_2) "NoCollision")
    (bind _returnvalue_3 (Transformation|AttachComponentToComponent _asbp_side_scroller_character_2 (Variables|Default|GetCube) "None" "SnapToTarget" "KeepRelative" "KeepWorld" false))
    (bind _output_get (Variables|Default|Setchar_snapped _returnvalue_3))
    (if _output_get
      (Input|RemoveMappingContext _returnvalue_2 "/Game/Bartender/Input/IMC_Default.IMC_Default" "(bIgnoreAllPressedKeysUntilRelease=True,bForceImmediately=False,bNotifyUserSettings=False)")
      (Input|AddMappingContext _returnvalue_2 "/Game/Bartender/Input/IMC_Cocos.IMC_Cocos" 1 "(bIgnoreAllPressedKeysUntilRelease=True,bForceImmediately=False,bNotifyUserSettings=False)")
      (Collision|SetCollisionEnabled (Variables|Default|GetCube) "NoCollision")
      (Default|GetState _asbp_side_scroller_character "NewEnumerator3")
      (Collision|SetCollisionEnabled (Variables|/Script/Engine.Character|GetCapsuleComponent _asbp_side_scroller_character) "QueryOnly")
      (Development|PrintString "that is my boy"))))

(event EventBeginPlay
  (bind _throw_params (Variables|Default|GetThrow_Params))
  (Variables|/Game/AdvancedSideScrollerTemplate/Blueprints/Character/BP_SideScrollerCharacter.BP_SideScrollerCharacter_C|SetCocos_ref (.AsBP%20Side%20Scroller%20Character (Utilities|Casting|CastToBP_SideScrollerCharacter (.main_character _throw_params))) self)
  (if (.isenchanted _throw_params)
    (Physics|SetPhysicsLinearVelocity (Variables|Default|GetCocos_ball_mesh) (Math|Vector|MakeVector 0.0 (.y (Variables|Default|Getoutside_force)) 0.0) false "None")
    ;[1 1 1] Life time
    (Utilities|FlowControl|RetriggerableDelay 1e+01)
    (Actor|DestroyActor)))

(event EventTick
  (params (DeltaSeconds :type Float%20%28single-precision%29))
  (bind _throw_params (Variables|Default|GetThrow_Params))
  (bind _cocos_ball_mesh (Variables|Default|GetCocos_ball_mesh))
  (bind _cube (Variables|Default|GetCube))
  (bind _returnvalue (Transformation|GetRelativeTransform _cocos_ball_mesh))
  (bind _returnvalue_2 (Transformation|GetWorldLocation _cube))
  (bind _asbp_side_scroller_character (Utilities|Casting|CastToBP_SideScrollerCharacter (.main_character _throw_params)))
  (Transformation|SetWorldLocation (Variables|Default|GetCube) (Math|Vector|MakeVector (.x (.location _returnvalue)) (.y (.location _returnvalue)) (+ (.z (.location _returnvalue)) (.SphereRadius (Collision|GetComponentBounds _cocos_ball_mesh)))) true false)
  ;[0.9561 0.9534 1] Locking character's location on snapping
  (if (Variables|Default|Getchar_snapped)
    (Transformation|SetActorLocation _asbp_side_scroller_character (Math|Vector|MakeVector (.x _returnvalue_2) (.y _returnvalue_2) (+ (.z _returnvalue_2) (.z (.BoxExtent (Collision|GetComponentBounds (Variables|/Script/Engine.Character|GetMesh _asbp_side_scroller_character)))))) false false)
    ;[1 1 1] Disable character's falling
    (Variables|/Script/Engine.MovementComponent|SetVelocity (Variables|/Script/Engine.Character|GetCharacterMovement _asbp_side_scroller_character) "0, 0, 0")
    ;[1 1 1] Life time
    (Utilities|FlowControl|RetriggerableDelay 1e+01)
    (Actor|DestroyActor)))

(fn ConstructionScript)

(fn GetState
  (params (state :type ActionState_E%20Enum :default "NewEnumerator0")))

(fn GetCharacterReference
  (return 0))

(fn GetCutsceneData
  (return 0.0 false))

(fn GetHealthVariables
  (return 0.0 0.0 0.0))

(fn GetInteractionVariables
  (return 0.0 false 0))

(fn GetMovementVariables
  (return false false false false 0.0 0.0 false 0.0 false))
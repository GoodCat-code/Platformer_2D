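; BP_Throw is a cocktail throw projectile that turns into a BP_Cocos actor, the only cocktail type handled here.
; On BeginPlay it drops straight down, or in the enhanced version flies along the player's forward Y and spawns after a short delay.
; Overlapping a static mesh also triggers the spawn.
; Spawning clears existing BP_Cocos, passes throw settings and velocity to a randomly rotated new one, then destroys the projectile.
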(event OnComponentBeginOverlap(Sphere)
  (params (OverlappedComponent :type Primitive%20Component%20Object%20Reference) (OtherActor :type Actor%20Object%20Reference) (OtherComp :type Primitive%20Component%20Object%20Reference) (OtherBodyIndex :type Integer) (bFromSweep :type Boolean) (SweepResult :type Hit%20Result%20Structure%20%28by%20ref%29))
  (bind _returnvalue (Transformation|GetActorLocation))
  (bind _returnvalue_2 (Math|Random|RandomFloatinRange 0.0 3.6e+02))
  (Utilities|Casting|CastToStaticMeshComponent OtherComp)
  (switch Utilities|FlowControl|Switch|SwitchonE_Coctails (.coctail (Variables|Default|GetS_throw_settings))
    (:NewEnumerator0
      ;[1 1 1] check cocos is exist
      (bind _outactors (Actor|GetAllActorsOfClass "/Game/Bartender/Blueprints/Coctails_bp/Cocos/BP_Cocos.BP_Cocos_C"))
      (if (Utilities|Array|IsNotEmpty _outactors)
        (Actor|DestroyActor _outactors))
      (Game|SpawnActorfromClass "/Game/Bartender/Blueprints/Coctails_bp/Cocos/BP_Cocos.BP_Cocos_C" (Math|Transform|MakeTransform (Math|Vector|MakeVector (.x _returnvalue) (.y _returnvalue) (+ (.z _returnvalue) 5e+01)) (Math|Rotator|MakeRotator 0.0 _returnvalue_2 _returnvalue_2) "1.000000,1.000000,1.000000") "AlwaysSpawn" "MultiplyWithRoot" 0 (Variables|Default|GetS_throw_settings) (Transformation|GetVelocity) 0)
      (Actor|DestroyActor))))

(event Custom|Force_Spawn
  (bind _returnvalue (Transformation|GetActorLocation))
  (bind _returnvalue_2 (Math|Random|RandomFloatinRange 0.0 3.6e+02))
  ;[1 1 1] check cocos is exist
  (bind _outactors (Actor|GetAllActorsOfClass "/Game/Bartender/Blueprints/Coctails_bp/Cocos/BP_Cocos.BP_Cocos_C"))
  (if (Utilities|Array|IsNotEmpty _outactors)
    (Actor|DestroyActor _outactors))
  (Game|SpawnActorfromClass "/Game/Bartender/Blueprints/Coctails_bp/Cocos/BP_Cocos.BP_Cocos_C" (Math|Transform|MakeTransform (Math|Vector|MakeVector (.x _returnvalue) (.y _returnvalue) (+ (.z _returnvalue) 5e+01)) (Math|Rotator|MakeRotator 0.0 _returnvalue_2 _returnvalue_2) "1.000000,1.000000,1.000000") "AlwaysSpawn" "MultiplyWithRoot" 0 (Variables|Default|GetS_throw_settings) (Transformation|GetVelocity) 0)
  (Actor|DestroyActor))

(event EventBeginPlay
  (bind _s_throw_settings (Variables|Default|GetS_throw_settings))
  (switch Utilities|FlowControl|Switch|SwitchonE_Coctails (.coctail _s_throw_settings)
    (:NewEnumerator0
      (if (.enhanced_version _s_throw_settings)
        (Variables|/Script/Engine.MovementComponent|SetVelocity (Variables|Default|GetProjectileMovement) (Math|Vector|MakeVector 0.0 (* (.y (Transformation|GetActorForwardVector (Game|GetPlayerCharacter 0))) 1e+03) 0.0))
        (Utilities|FlowControl|Delay 0.3)
        (CallFunction|ForceSpawn)
        (else
          (Variables|/Script/Engine.MovementComponent|SetVelocity (Variables|Default|GetProjectileMovement) "0.000000,0.000000,-5000.000000"))))))

(fn ConstructionScript)